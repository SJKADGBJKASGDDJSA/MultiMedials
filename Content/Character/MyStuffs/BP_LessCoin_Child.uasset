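; BP_LessCoin_Child is a child Blueprint for a penalty coin that takes one from BP_PersonajeExotico's Coin count on overlap.
; Begin overlap prints the new count in red, disables Collider collision and calls A2, which is not defined here.
; End overlap hides the actor and Collider.
; A custom event, with no caller here, uses a two-second retriggerable delay before unhiding the actor and restoring query-only collision.
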(event `self.Collider.OnComponentEndOverlap`
  (params (OverlappedComponent :type "PrimitiveComponent Object Reference") (OtherActor :type "Actor Object Reference") (OtherComp :type "PrimitiveComponent Object Reference") (OtherBodyIndex :type Integer))
  ;[0 0.009911 0.03125] Destruir monedas
  (cast `/Game/Character/BP_PersonajeExotico` OtherActor)
  (`self.SetActorHiddenInGame` self true)
  (`SceneComponent.SetHiddenInGame` (`self.Collider`) true false))

(event `self.Collider.OnComponentBeginOverlap`
  (params (OverlappedComponent :type "PrimitiveComponent Object Reference") (OtherActor :type "Actor Object Reference") (OtherComp :type "PrimitiveComponent Object Reference") (OtherBodyIndex :type Integer) (bFromSweep :type Boolean) (SweepResult :type "HitResult Structure (by ref)"))
  ;[0.02317 0.005714 0.03125] Contador de monedas
  (bind _asbp_personaje_exotico (cast `/Game/Character/BP_PersonajeExotico` OtherActor))
  (bind _output_get (set `/Game/Character/BP_PersonajeExotico.Coin` (- (`/Game/Character/BP_PersonajeExotico.Coin` _asbp_personaje_exotico) 1.0) _asbp_personaje_exotico))
  (`KismetSystemLibrary.PrintString` (`KismetStringLibrary.Conv_DoubleToString` _output_get) true true (struct :`R` 1.0 :`G` 0.110692 :`A` 1.0))
  (`self.SetActorHiddenInGame` false)
  (`PrimitiveComponent.SetCollisionEnabled` (`self.Collider`) "NoCollision")
  (`self.a2`))

(event `CustomEvent`
  ;[0.01874 0.03125 0.001865] Aparecer y Desaparecer
  (`KismetSystemLibrary.RetriggerableDelay` 2.0)
  (`self.SetActorHiddenInGame` false)
  (`PrimitiveComponent.SetCollisionEnabled` (`self.Collider`) "QueryOnly"))

(fn `UserConstructionScript`
  (`parent.UserConstructionScript`))